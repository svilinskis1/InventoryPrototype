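; Dialogue character Blueprint that lets the player talk to it with E while nearby.
; InteractionRadius overlaps toggle the TalkLabel prompt, and the key press checks the player capsule is inside before calling Talk.
; Talk increments TalkIndex through InitialDialog, or RepeatDialog once Interacted is set, using a DialogBox widget for text.
; Passing the last line removes the widget and resets the index, with the first completed conversation setting Interacted.
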(event OnComponentBeginOverlap(InteractionRadius)
  (params (OverlappedComponent :type Primitive%20Component%20Object%20Reference) (OtherActor :type Actor%20Object%20Reference) (OtherComp :type Primitive%20Component%20Object%20Reference) (OtherBodyIndex :type Integer) (bFromSweep :type Boolean) (SweepResult :type Hit%20Result%20Structure%20%28by%20ref%29))
  ;[0.15 0.15 0.15 0.5] Show/hide talk text when player in range
  (Rendering|SetVisibility (Variables|Default|GetTalkLabel) true false))

(event OnComponentEndOverlap(InteractionRadius)
  (params (OverlappedComponent :type Primitive%20Component%20Object%20Reference) (OtherActor :type Actor%20Object%20Reference) (OtherComp :type Primitive%20Component%20Object%20Reference) (OtherBodyIndex :type Integer))
  ;[0.15 0.15 0.15 0.5] Show/hide talk text when player in range
  (Rendering|SetVisibility (Variables|Default|GetTalkLabel) false false))

(event Custom|Talk
  ;[0.15 0.15 0.15 0.5] Talk by looping through dialog options
  (Math|Integer|IncrementInt (Variables|Default|GetTalkIndex)
    (:%20%20
      (if (Variables|Default|GetInteracted)
        (if (< (Variables|Default|GetTalkIndex) (Utilities|Array|Length (Variables|Default|GetRepeatDialog)))
          (Variables|Default|GetDialogBox
            (:then)
            (:else
              (UserInterface|CreateWidget "/Game/UI/WB_DialogBox.WB_DialogBox_C" (Game|GetPlayerController 0))
              (Rendering|Components|TextRender|SetText (Variables|/Game/UI/WB_DialogBox.WB_DialogBox_C|GetDialogText (Variables|Default|GetDialogBox)) (Utilities|Text|ToText(String) (Utilities|Array|Get(acopy) (Variables|Default|GetRepeatDialog) (Variables|Default|GetTalkIndex))))))
          (else
            (Widget|RemovefromParent (Variables|Default|GetDialogBox))
            (Variables|Default|SetTalkIndex -1)))
        (elif (< (Variables|Default|GetTalkIndex) (Utilities|Array|Length (Variables|Default|GetInitialDialog)))
          (Variables|Default|GetDialogBox
            (:then)
            (:else
              (bind _returnvalue (UserInterface|CreateWidget "/Game/UI/WB_DialogBox.WB_DialogBox_C" (Game|GetPlayerController 0)))
              (Variables|Default|SetDialogBox _returnvalue)
              (Rendering|Components|TextRender|SetText (Variables|/Game/UI/WB_DialogBox.WB_DialogBox_C|GetDialogText (Variables|Default|GetDialogBox)) (Utilities|Text|ToText(String) (Utilities|Array|Get(acopy) (Variables|Default|GetInitialDialog) (Variables|Default|GetTalkIndex))))))
          (else
            (Widget|RemovefromParent (Variables|Default|GetDialogBox))
            (Variables|Default|SetTalkIndex -1)
            (Variables|Default|SetInteracted true)))))))

(event Input|KeyboardEvents|E
  (params (Key :type Key%20Structure :default "None"))
  ;[0.15 0.15 0.15 0.5] Start talking when E pressed
  (:Pressed
    (if (Class|PrimitiveComponent|IsOverlappingComponent (Variables|Default|GetInteractionRadius) (Variables|/Script/Engine.Character|GetCapsuleComponent (Game|GetPlayerCharacter 0)))
      (CallFunction|Talk self))))

(fn ConstructionScript)