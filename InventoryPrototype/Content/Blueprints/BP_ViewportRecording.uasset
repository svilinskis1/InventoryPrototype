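; Item preview actor that renders a mesh through a scene capture for the inventory screen's viewport.
; The SceneCaptureComponent2D shows only ItemMesh; UpdateMesh swaps the mesh, resets rotation and camera position, then calls LoadViewport on the player's inventory screen.
; Mouse events rotate the mesh by scaled drag delta, set CanRotate on click only when Is3D, and zoom by offsetting the capture's location.
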(event Custom|ClickStart
  (params (ClickPosition :type Vector%202D%20Structure))
  ;[0.15 0.15 0.15 0.5] Start rotating when player clicks
  (Variables|Default|SetClickPosition ClickPosition)
  (if (Variables|Default|Getis3D)
    (Variables|Default|SetCanRotate true)))

(event Custom|ClickEnd
  ;[0.15 0.15 0.15 0.5] Stop rotating when player stops clicking
  (Variables|Default|SetCanRotate false))

(event Custom|MouseMoved
  (params (MousePosition :type Vector%202D%20Structure))
  ;[0.15 0.15 0.15 0.5] Rotate object when mouse moves
  (Transformation|AddWorldRotation (Variables|Default|GetItemMesh) (Math|Rotator|MakeRotator 0.0 (.Y (Math|Vector2D|BreakVector2D (/ (- MousePosition (Variables|Default|GetClickPosition)) "(X=5.000000,Y=5.000000)"))) (* (.X (Math|Vector2D|BreakVector2D (/ (- MousePosition (Variables|Default|GetClickPosition)) "(X=5.000000,Y=5.000000)"))) -1.0)) false false)
  (Variables|Default|SetClickPosition MousePosition))

(event Custom|Zoom
  (params (Amount :type Vector))
  (bind _scenecapturecomponent2d (Variables|Default|GetSceneCaptureComponent2D))
  ;[0.15 0.15 0.15 0.5] Zoom in and out
  (Transformation|SetRelativeLocation _scenecapturecomponent2d (+ Amount (Variables|/Script/Engine.SceneComponent|GetRelativeLocation _scenecapturecomponent2d)) false false))

(event EventBeginPlay
  (Rendering|SceneCapture|ShowOnlyComponent (Variables|Default|GetSceneCaptureComponent2D) (Variables|Default|GetItemMesh)))

(fn ConstructionScript)

(fn UpdateMesh
  (params (NewMesh :type Static%20Mesh%20Object%20Reference))
  (bind _itemmesh (Variables|Default|GetItemMesh))
  (Components|StaticMesh|SetStaticMesh _itemmesh NewMesh)
  ;[0.15 0.15 0.15 0.5] Reset viewport
  (Rendering|SetVisibility _itemmesh true false)
  (Transformation|SetWorldRotation (Variables|Default|GetItemMesh) "0, 0, 0" false false)
  (Transformation|SetRelativeLocation (Variables|Default|GetSceneCaptureComponent2D) "-220.000000,0.000000,50.000000" false true)
  (Default|LoadViewport (Variables|/Game/Blueprints/AC_InventoryConstruct.AC_InventoryConstruct_C|GetInventoryScreen (Actor|GetComponentbyClass (Game|GetPlayerCharacter 0) "/Game/Blueprints/AC_InventoryConstruct.AC_InventoryConstruct_C"))))