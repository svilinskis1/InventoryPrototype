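; Inventory component that holds an item list and toggles a pause-menu inventory screen with Escape.
; Opening creates a fresh WB_InventoryScreen loaded from the component and pauses the game; closing removes it and unpauses, leaving the mouse cursor visible.
; AddItem and RemoveItem edit the list and immediately reload the screen.
; BeginPlay also spawns a BP_ViewportRecording actor far outside the play space and stores it as Recorder.
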(event EventBeginPlay
  (bind _returnvalue (Game|SpawnActorfromClass "/Game/Blueprints/BP_ViewportRecording.BP_ViewportRecording_C" (Math|Transform|MakeTransform "-999999.000000,0.000000,0.000000") "Undefined" "MultiplyWithRoot" 0 0))
  (Variables|Default|SetRecorder _returnvalue))

(event Input|KeyboardEvents|Escape
  (params (Key :type Key%20Structure :default "None"))
  (:Pressed
    (if (Widget|IsVisible (Variables|Default|GetInventoryScreen))
      ;[0.15 0.15 0.15 0.5] hide inventory
      (Widget|RemovefromParent (Variables|Default|GetInventoryScreen))
      (Game|SetGamePaused false)
      (Variables|/Script/Engine.PlayerController|SetbShowMouseCursor (Game|GetPlayerController 0) true)
      (else
        ;[0.15 0.15 0.15 0.5] show inventory
        (bind _returnvalue (UserInterface|CreateWidget "/Game/UI/WB_InventoryScreen.WB_InventoryScreen_C"))
        (bind _output_get (Variables|Default|SetInventoryScreen _returnvalue))
        (Default|LoadInventoryItems (Variables|Default|GetInventoryScreen) self)
        (UserInterface|Viewport|AddtoViewport _output_get 0)
        (Game|SetGamePaused true)
        (Variables|/Script/Engine.PlayerController|SetbShowMouseCursor (Game|GetPlayerController 0) true)))))

(fn AddItem
  (params (ItemInfo :type F%20Item%20Struct%20Structure))
  (Utilities|Array|Add (Variables|Default|GetItems) ItemInfo)
  (Default|LoadInventoryItems (Variables|Default|GetInventoryScreen) self))

(fn RemoveItem
  (params (Item :type F%20Item%20Struct%20Structure))
  (Utilities|Array|RemoveItem (Variables|Default|GetItems) Item)
  (Default|LoadInventoryItems (Variables|Default|GetInventoryScreen) self))