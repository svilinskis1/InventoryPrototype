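; Item is a pickup actor that the player collects into their inventory with the E key.
; Overlap events on CollectionRadius show and hide ControlsLabel as a prompt, without filtering which component overlaps.
; On E, it checks that the player capsule overlaps the radius and the InventoryConstruct component has room under a hardcoded five-item cap.
; It then passes ItemInfo to AddItem and destroys itself.
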(event OnComponentBeginOverlap(CollectionRadius)
  (params (OverlappedComponent :type Primitive%20Component%20Object%20Reference) (OtherActor :type Actor%20Object%20Reference) (OtherComp :type Primitive%20Component%20Object%20Reference) (OtherBodyIndex :type Integer) (bFromSweep :type Boolean) (SweepResult :type Hit%20Result%20Structure%20%28by%20ref%29))
  ;[0.15 0.15 0.15 0.5] Show/hide tooltip when player in range
  (Rendering|SetVisibility (Variables|Default|GetControlsLabel) true false))

(event OnComponentEndOverlap(CollectionRadius)
  (params (OverlappedComponent :type Primitive%20Component%20Object%20Reference) (OtherActor :type Actor%20Object%20Reference) (OtherComp :type Primitive%20Component%20Object%20Reference) (OtherBodyIndex :type Integer))
  ;[0.15 0.15 0.15 0.5] Show/hide tooltip when player in range
  (Rendering|SetVisibility (Variables|Default|GetControlsLabel) false false))

(event Input|KeyboardEvents|E
  (params (Key :type Key%20Structure :default "None"))
  (bind _returnvalue (Game|GetPlayerCharacter 0))
  (bind _returnvalue_2 (Actor|GetComponentbyClass _returnvalue "/Game/Blueprints/InventoryConstruct.InventoryConstruct_C"))
  ;[0.15 0.15 0.15 0.5] Add object to inventory when E pressed
  (:Pressed
    (if (Class|PrimitiveComponent|IsOverlappingComponent (Variables|Default|GetCollectionRadius) (Variables|/Script/Engine.Character|GetCapsuleComponent _returnvalue))
      (if (<= (Utilities|Array|Length (Variables|/Game/Blueprints/InventoryConstruct.InventoryConstruct_C|GetItems _returnvalue_2)) 4)
        (Default|AddItem _returnvalue_2 (Variables|Default|GetItemInfo))
        (Actor|DestroyActor)))))

(fn ConstructionScript)