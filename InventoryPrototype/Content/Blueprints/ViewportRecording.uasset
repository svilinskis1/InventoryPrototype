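; Preview actor that captures an item mesh in isolation with a SceneCaptureComponent2D, with drag rotation and zoom.
; BeginPlay adds the mesh to the capture's show-only list.
; ClickStart and ClickEnd gate MouseMoved, which feeds the passed position directly into world yaw (inverted X) and pitch (Y).
; Zoom offsets the capture's relative location, and UpdateMesh calls SetStaticMesh with no mesh specified.
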(event Custom|ClickStart
  (params (ClickPosition :type Vector%202D%20Structure))
  (Variables|Default|SetClickPosition ClickPosition)
  (Variables|Default|SetCanRotate true))

(event Custom|ClickEnd
  (Variables|Default|SetCanRotate false))

(event Custom|MouseMoved
  (params (MousePosition :type Vector%202D%20Structure))
  (bind (_x _y) (Math|Vector2D|BreakVector2D MousePosition))
  (if (Variables|Default|GetCanRotate)
    (Transformation|AddWorldRotation (Variables|Default|GetItemMesh) (Math|Rotator|MakeRotator 0.0 _y (* _x -1.0)) false false)
    (Variables|Default|SetClickPosition MousePosition)))

(event Custom|Zoom
  (params (Amount :type Vector))
  (bind _scenecapturecomponent2d (Variables|Default|GetSceneCaptureComponent2D))
  (Transformation|SetRelativeLocation _scenecapturecomponent2d (+ Amount (Variables|/Script/Engine.SceneComponent|GetRelativeLocation _scenecapturecomponent2d)) false false))

(event EventBeginPlay
  (Rendering|SceneCapture|ShowOnlyComponent (Variables|Default|GetSceneCaptureComponent2D) (Variables|Default|GetItemMesh)))

(fn ConstructionScript)

(fn UpdateMesh
  (Components|StaticMesh|SetStaticMesh (Variables|Default|GetItemMesh) 0))